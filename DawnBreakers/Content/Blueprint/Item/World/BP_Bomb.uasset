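; BP_Bomb is a damageable world bomb that explodes once incoming damage depletes its HP.
; The construction script gathers nine particle systems into Effects, and AnyDamage subtracts truncated damage from HP while it is above zero.
; On depletion, a loop activates each effect, hides the mesh and text, disables mesh collision responses, and applies full-strength radial damage, so that damage repeats once per effect.
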(event EventBeginPlay)

(event Collision|EventActorBeginOverlap
  (params (OtherActor :type Actor%20Object%20Reference)))

(event Game|Damage|EventAnyDamage
  (params (Damage :type Float%20%28single-precision%29) (DamageType :type Damage%20Type%20Object%20Reference) (InstigatedBy :type Controller%20Object%20Reference) (DamageCauser :type Actor%20Object%20Reference))
  (bind _staticmesh (Variables|Default|GetStaticMesh))
  (if (> (Variables|Default|GetHP) 0)
    (bind _output_get (Variables|Default|SetHP (- (stale _output_get) (Math|Float|Truncate Damage))))
    (if (<= _output_get 0)
      (for _array_element (Variables|Default|GetEffects)
        (Components|Activation|SetActive _array_element true true)
        (Rendering|SetVisibility _staticmesh false false)
        (Collision|SetCollisionResponsetoAllChannels _staticmesh "ECR_Ignore")
        (Rendering|SetVisibility (Variables|Default|GetTextRender) false false)
        (Game|Damage|ApplyRadialDamage 1.5e+03 (Transformation|GetWorldLocation (Variables|Default|GetStaticMesh)) 1e+03 "/Script/Engine.DamageType" 0 0 0 true "ECC_Visibility")))))

(event EventTick
  (params (DeltaSeconds :type Float%20%28single-precision%29)))

(fn ConstructionScript
  (Variables|Default|SetEffects (Utilities|Array|MakeArray (Variables|Default|GetParticleSystem1) (Variables|Default|GetParticleSystem5) (Variables|Default|GetParticleSystem6) (Variables|Default|GetParticleSystem8) (Variables|Default|GetParticleSystem3) (Variables|Default|GetParticleSystem2) (Variables|Default|GetParticleSystem7) (Variables|Default|GetParticleSystem4) (Variables|Default|GetParticleSystem))))