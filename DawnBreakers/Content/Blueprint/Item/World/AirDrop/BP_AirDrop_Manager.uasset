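; Air drop manager that validates a requested drop point and sends a Chinook helicopter to make the drop.
; Validation optionally line-traces down for a flat enough surface and box-traces up for clear sky.
; The authority spawns the Chinook on a random circle around the manager at drop height, with the opposite point as exit.
; Remote callers forward the request through ServerAttemptDrop and return their local validity check.
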(event Custom|ServerAttemptDrop
  (params (DesiredDropPoint :type Vector))
  (CallFunction|AttemptDrop DesiredDropPoint))

(event EventBeginPlay)

(fn ConstructionScript)

(fn IsDropPointValid
  (params (DropLocation :type Vector) (OptionalUpVector :type Vector))
  (bind _verticalscanextentradius (Variables|Config|GetVerticalScanExtentRadius))
  ;[1 1 1] Store local copies of function input so we don't need wires everywhere
  (LocalVariables|SetLocalDropLocation DropLocation)
  (LocalVariables|SetLocalUpVector (Math|Vector|SelectVector OptionalUpVector "0, 0,1.000000" (> (Math|Vector|VectorLengthSquared OptionalUpVector) 0.0)))
  (Utilities|FlowControl|Sequence
    (:then_0
      ;[1 1 1] If DoAngleCheck is enabled, we will see if our drop point is above a valid drop surface with a suitable surface angle
      (if (Variables|Config|GetbDoAngleCheck)
        (bind (_outhit _returnvalue) (Collision|LineTraceByChannel (LocalVariables|GetLocalDropLocation) (- (LocalVariables|GetLocalDropLocation) (* (LocalVariables|GetLocalUpVector) (Variables|Config|GetStartVerticalScanOffset))) "TraceTypeQuery1" false 0 "None"))
        (if _returnvalue
          (if (>= (Math|Vector|DotProduct (.ImpactNormal (Collision|BreakHitResult _outhit)) "0, 0,1.000000") (Variables|Config|GetValidDotUpAngle))
            ;[1 1 1] Do a vertical box trace to see if there is anything above us...
            (if (Variables|Config|GetbDoClearSkyCheck) :!label _label
              (bind _returnvalue_2 (Collision|BoxTraceByChannel (+ (LocalVariables|GetLocalDropLocation) (Math|Vector|MakeVector 0.0 0.0 (Variables|Config|GetStartVerticalScanOffset))) (+ (+ (LocalVariables|GetLocalDropLocation) (Math|Vector|MakeVector 0.0 0.0 (Variables|Config|GetStartVerticalScanOffset))) (Math|Vector|MakeVector 0.0 0.0 (Variables|Config|GetDropHeight))) (Math|Vector|MakeVector _verticalscanextentradius _verticalscanextentradius 0.0) "0, 0,0.000000" "TraceTypeQuery1" false 0 "None"))
              (if (not _returnvalue_2)
                (LocalVariables|SetIsValidDropLocation true :!label _label_2)
                (else
                  (LocalVariables|SetIsValidDropLocation false :!label _label_3)))
              (else
                (goto _label_2)))
            (else
              (goto _label_3)))
          (else
            (goto _label_3)))
        (else
          (goto _label))))
    (:then_1
      ;[1 1 1] Return whether this drop location is valid
      (return (LocalVariables|GetIsValidDropLocation)))))

(fn AttemptDrop
  (params (DesiredDropPoint :type Vector))
  (bind _returnvalue (Transformation|GetActorLocation))
  (bind _dropheight (Variables|Config|GetDropHeight))
  (bind _returnvalue_2 (Math|Vector|MakeVector 0.0 0.0 _dropheight))
  (bind _returnvalue_3 (+ _returnvalue _returnvalue_2))
  (LocalVariables|SetLocalDropPoint DesiredDropPoint) ; Copy of Desired Drop Point so we don't need wires everywhere
  (Networking|SwitchHasAuthority
    (:Authority
      (bind _bisvalid (CallFunction|IsDropPointValid (LocalVariables|GetLocalDropPoint) "0, 0, 0"))
      (if _bisvalid
        (LocalVariables|SetCircleOffsetForPath (* (Math|Vector|Normalize (* (Math|Random|RandomUnitVector) "1.000000,1.000000,0.000000")) (Variables|Config|GetHeloSpawnRadius)))
        (Game|SpawnActorfromClass "/Game/Blueprint/Item/World/AirDrop/Chinook/BP_AirDrop_Chinook.BP_AirDrop_Chinook_C" (Math|Transform|MakeTransform (+ _returnvalue_3 (LocalVariables|GetCircleOffsetForPath)) (Math|Rotator|MakeRotfromX (- (+ _returnvalue_3 (LocalVariables|GetCircleOffsetForPath)) (+ (LocalVariables|GetLocalDropPoint) (Math|Vector|MakeVector 0.0 0.0 (Variables|Config|GetDropHeight)))))) "AlwaysSpawn" 0 (+ (LocalVariables|GetLocalDropPoint) (Math|Vector|MakeVector 0.0 0.0 (Variables|Config|GetDropHeight))) (+ _returnvalue_3 (* (LocalVariables|GetCircleOffsetForPath) -1.0)))
        (return true)
        (else
          (return false))))
    (:Remote
      (CallFunction|ServerAttemptDrop (LocalVariables|GetLocalDropPoint))
      (bind _bisvalid_2 (CallFunction|IsDropPointValid (LocalVariables|GetLocalDropPoint) "0.000000, 0, 0"))
      (return _bisvalid_2))))