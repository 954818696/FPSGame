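; Chinook air drop actor that flies to a target location, spawns a BP_AirDropPackage at its DropPoint, then flies to a leave location and destroys itself.
; PrepareTravelToPoint records the start location, start time and a distance-over-speed duration for each leg.
; On Tick, the server alone moves it with a time-based EaseInOut interpolation, using the Dropped flag to switch destinations and trigger the drop or cleanup.
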(event EventBeginPlay
  (CallFunction|PrepareTraveltoPoint (Variables|Config|GetTargetDropLocation)))

(event EventTick
  (params (DeltaSeconds :type Float%20%28single-precision%29))
  (bind _returnvalue (Utilities|Time|GetGameTimeinSeconds))
  (bind _travelstarttime (Variables|Default|GetTravelStartTime))
  (bind _travelduration (Variables|Default|GetTravelDuration))
  (bind _returnvalue_2 (- _returnvalue _travelstarttime))
  (bind _returnvalue_3 (/ _returnvalue_2 _travelduration))
  (bind _returnvalue_4 (Math|Float|Clamp(Float) _returnvalue_3))
  (bind _returnvalue_5 (>= _returnvalue_4 1.0))
  ;[1 1 1] Handle traveling to destination over time
  (Networking|SwitchHasAuthority
    (:Authority
      (Transformation|SetActorLocation (Math|Interpolation|Ease "EaseInOut" _returnvalue_4 (Variables|Default|GetStartLocation) (Math|Vector|SelectVector (Variables|Config|GetLeaveLocation) (Variables|Config|GetTargetDropLocation) (Variables|Default|GetbDropped)) 1.5) false false)
      ;[1 1 1] Reached Drop Point, spawn Drop Package and prepare to leave
      (if (and _returnvalue_5 (not (Variables|Default|GetbDropped))) ; Reached Drop Point?
        (Game|SpawnActorfromClass "/Game/Blueprint/Item/World/AirDrop/BP_AirDropPackage.BP_AirDropPackage_C" (Math|Conversions|ToTransform(Vector) (Transformation|GetWorldLocation (Variables|Default|GetDropPoint))) "Undefined" 0 0)
        (Variables|Default|SetbDropped true)
        (CallFunction|PrepareTraveltoPoint (Variables|Config|GetLeaveLocation))
        (else
          ;[1 1 1] Destroy ourselves if we've reached the leave point
          (if (and _returnvalue_5 (Variables|Default|GetbDropped)) ; Reached Leave Point?
            (Actor|DestroyActor)))))))

(fn ConstructionScript)

(fn PrepareTraveltoPoint
  (params (Destination :type Vector))
  (bind _output_get (Variables|Default|SetStartLocation (Transformation|GetActorLocation))) ; Store where we start from
  (Variables|Default|SetTravelDuration (/ (Math|Vector|VectorLength (- Destination _output_get)) (Variables|Default|GetSpeed))) ; Store how long it takes to get there
  (Variables|Default|SetTravelStartTime (Utilities|Time|GetGameTimeinSeconds)) ; Store when we started traveling
  (return))