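; BP_DayLighting is a world weather actor that links the level's sun and sky lighting and keeps the sky sphere's sun direction current.
; On BeginPlay it finds and caches the BP_Sky_Sphere, DirectionalLight and SkyLight, printing a message if missing and assigning only when exactly one exists.
; Each Tick runs the parent tick, then calls UpdateSunDirection on the sky sphere without a validity check.
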(event EventBeginPlay
  (Utilities|FlowControl|Sequence
    (:then_0
      (bind _outactors (Actor|GetAllActorsOfClass "/Engine/EngineSky/BP_Sky_Sphere.BP_Sky_Sphere_C"))
      (if (== (Utilities|Array|Length _outactors) 0)
        (Development|PrintString "BP_SKySPhere not  found in BP_DayLighting.")
        (elif (== (Utilities|Array|Length _outactors) 1)
          (Variables|Default|SetBP_SkySphere (Utilities|Array|Get(acopy) _outactors)))))
    (:then_1
      (bind _outactors_2 (Actor|GetAllActorsOfClass "/Script/Engine.DirectionalLight"))
      (if (== (Utilities|Array|Length _outactors_2) 0)
        (Development|PrintString "DirectionalLight not found in BP_DayLighting.")
        (elif (== (Utilities|Array|Length _outactors_2) 1)
          (Variables|Default|SetmPrimarySunLight (Utilities|Array|Get(acopy) _outactors_2)))))
    (:then_2
      (bind _outactors_3 (Actor|GetAllActorsOfClass "/Script/Engine.SkyLight"))
      (if (== (Utilities|Array|Length _outactors_3) 0)
        (Development|PrintString "SkyLight not found in BP_DayLighting.")
        (elif (== (Utilities|Array|Length _outactors_3) 1)
          (Variables|Default|SetmSkyLight (Utilities|Array|Get(acopy) _outactors_3)))))))

(event EventActorBeginOverlap
  (params (OtherActor :type Actor%20Object%20Reference)))

(event EventTick
  (params (DeltaSeconds :type Float%20%28single-precision%29))
  ;[1 0.5662 0.754] 更新skyBp里太阳光位置
  (|CallParentFunction DeltaSeconds)
  (Default|UpdateSunDirection (Variables|Default|GetBP_SkySphere)))

(fn ConstructionScript)