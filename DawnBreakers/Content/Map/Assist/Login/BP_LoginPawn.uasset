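; Login pawn that drives mouse interaction with the 3D start scene menu and its options menu.
; BeginPlay shows the cursor, sets UI-only input and finds both menu actors.
; Each tick traces under the cursor, forwards hovered box components to the menus, plays a sound when the hover changes and clears it when neither is hit.
; Left click sends the last hovered box to the current menu.
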(event EventBeginPlay
  ;[1 1 1] Show Mouse
  (Variables|/Script/Engine.PlayerController|SetbShowMouseCursor (Game|GetPlayerController 0) true)
  (Input|SetInputModeUIOnly 0 0 "DoNotLock")
  (bind _outactors (Actor|GetAllActorsOfClass "/Game/Blueprint/UI/Lobby/BP_StartSceneMenu.BP_StartSceneMenu_C"))
  (Variables|Default|SetStartSceneMenu (Utilities|Array|Get(acopy) _outactors))
  (bind _outactors_2 (Actor|GetAllActorsOfClass "/Game/Blueprint/UI/Lobby/BP_StartSceneMenu_Options.BP_StartSceneMenu_Options_C"))
  (Variables|Default|SetOptionMenu (Utilities|Array|Get(acopy) _outactors_2))
  (Actor|Tick|SetActorTickEnabled self true))

(event EventTick
  (params (DeltaSeconds :type Float%20%28single-precision%29))
  (bind _returnvalue (Game|GetPlayerController 0))
  (bind _startscenemenu (Variables|Default|GetStartSceneMenu))
  (bind _optionmenu (Variables|Default|GetOptionMenu))
  (bind _hitresult (Game|Player|GetHitResultUnderCursorbyChannel _returnvalue "TraceTypeQuery1" true))
  (bind (_bblockinghit _binitialoverlap _time _location _impactpoint _normal _impactnormal _physmat _hitactor _hitcomponent) (Collision|BreakHitResult _hitresult))
  ;[1 1 1] MouseMove
  (Variables|Default|SetClearLastCount 0)
  (Utilities|FlowControl|Sequence
    (:then_0
      ;[1 1 1] MainMenu
      (bind _asbp_start_scene_menu (Utilities|Casting|CastToBP_StartSceneMenu _hitactor)
        (:then
          (bind _asbox_collision (Utilities|Casting|CastToBoxComponent _hitcomponent))
          (Default|BeginOverlap _asbp_start_scene_menu _asbox_collision)
          (if (not (== (Variables|Default|GetLastHitBox) _asbox_collision))
            (Audio|PlaySoundatLocation "/Game/ArtResource/Sound/InterfaceAudio/Stereo/MenuCursor_Sides_Stereo_Cue.MenuCursor_Sides_Stereo_Cue" (Transformation|GetActorLocation self))
            (Variables|Default|SetLastHitBox _asbox_collision)
            (Variables|Default|SetCurrentMenuIndex 0)))
        (:CastFailed
          (Utilities|IsValid _startscenemenu
            (:Is%20Valid
              (Default|EndOverlap _startscenemenu)
              (bind _output_get (Variables|Default|SetClearLastCount (+ (stale _output_get) 1))))))))
    (:then_1
      ;[1 1 1] OptionMenu
      (bind _asbp_start_scene_menu_options (Utilities|Casting|CastToBP_StartSceneMenu_Options _hitactor)
        (:then
          (bind _asbox_collision_2 (Utilities|Casting|CastToBoxComponent _hitcomponent))
          (Default|BeginOverlap _asbp_start_scene_menu_options _asbox_collision_2)
          (if (not (== (Variables|Default|GetLastHitBox) _asbox_collision_2))
            (Audio|PlaySoundatLocation "/Game/ArtResource/Sound/InterfaceAudio/Stereo/MenuCursor_Sides_Stereo_Cue.MenuCursor_Sides_Stereo_Cue" (Transformation|GetActorLocation self))
            (Variables|Default|SetLastHitBox _asbox_collision_2)
            (Variables|Default|SetCurrentMenuIndex 1)))
        (:CastFailed
          (Utilities|IsValid _optionmenu
            (:Is%20Valid
              (Default|EndOverlap _optionmenu)
              (bind _output_get_2 (Variables|Default|SetClearLastCount (+ (stale _output_get_2) 1))))))))
    (:then_2
      (if (== (Variables|Default|GetClearLastCount) 2)
        (Variables|Default|SetLastHitBox 0)))))

(event Input|MouseEvents|LeftMouseButton
  (params (Key :type Key%20Structure :default "AnyKey"))
  (bind _startscenemenu (Variables|Default|GetStartSceneMenu))
  (bind _optionmenu (Variables|Default|GetOptionMenu))
  ;[1 1 1] MouseClick
  (:Pressed
    (switch int (Variables|Default|GetCurrentMenuIndex)
      (:0
        ;[1 1 1] MainMenu
        (Utilities|IsValid _startscenemenu
          (:Is%20Valid
            (Default|OnClick _startscenemenu (Variables|Default|GetLastHitBox)))))
      (:1
        ;[1 1 1] OptionMenu
        (Utilities|IsValid _optionmenu
          (:Is%20Valid
            (Default|OnClick _optionmenu (Variables|Default|GetLastHitBox))))))))

(fn ConstructionScript)